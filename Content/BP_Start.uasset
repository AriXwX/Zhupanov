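; BP_Start is the start pad that procedurally builds a run of platforms for the third-person character.
; Beginning an overlap destroys the exit referenced by the character.
; When the character leaves, it spawns a BP_Death below, widened by Difficulty, and a lower chain of platforms whose count grows with Difficulty.
; Each platform is placed at a random X gap from the previous one, with a BP_Exit closing the chain.
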(event `self.ReceiveBeginPlay`
  (bind _returnvalue (`GameplayStatics.GetActorOfClass` "/Game/ThirdPersonBP/Blueprints/ThirdPersonCharacter.ThirdPersonCharacter_C"))
  (set `self.TPC` _returnvalue))

(event `self.ReceiveActorBeginOverlap`
  (params (OtherActor :type "Actor Object Reference"))
  (bind _as_bp_exit (`/Game/ThirdPersonBP/Blueprints/ThirdPersonCharacter.As BP Exit` (`self.TPC`)))
  (`/Engine/EditorBlueprintResources/StandardMacros.IsValid` _as_bp_exit
    (:`Is Valid`
      (`self.K2_DestroyActor` _as_bp_exit))))

(event `self.ReceiveActorEndOverlap`
  (params (OtherActor :type "Actor Object Reference"))
  (bind (_returnvalue_x _returnvalue_y _returnvalue_z) (`KismetMathLibrary.BreakVector` (`self.K2_GetActorLocation`)))
  (bind _platforms (`self.Platforms`))
  (bind _platforms_2 (`self.Platforms`))
  (bind (_returnvalue_x_2 _returnvalue_y_2 _returnvalue_z_2) (`KismetMathLibrary.BreakVector` (`self.K2_GetActorLocation` (`|GetArrayItem` _platforms (`KismetArrayLibrary.Array_LastIndex` _platforms)))))
  (bind (_returnvalue_x_3 _returnvalue_y_3 _returnvalue_z_3) (`KismetMathLibrary.BreakVector` (`self.K2_GetActorLocation` (`|GetArrayItem` _platforms_2 (`KismetArrayLibrary.Array_LastIndex` _platforms_2)))))
  (cast `/Game/ThirdPersonBP/Blueprints/ThirdPersonCharacter` OtherActor)
  (`|SpawnActorFromClass` "/Game/BP_Death.BP_Death_C" (`KismetMathLibrary.MakeTransform` (- (`self.K2_GetActorLocation`) (0.0 0.0 1000.0)) (struct) (`KismetMathLibrary.MakeVector` (`KismetMathLibrary.Conv_IntToDouble` (* (+ (`/Game/ThirdPersonBP/Blueprints/ThirdPersonCharacter.Difficulty` (`self.TPC`)) 4) 50)) 2.0 1.0)) "AlwaysSpawn" "OverrideRootScale" null null)
  (bind _returnvalue (`|SpawnActorFromClass` "/Game/BP_Platform.BP_Platform_C" (`KismetMathLibrary.MakeTransform` (`KismetMathLibrary.MakeVector` (+ (+ 600.0 _returnvalue_x) (`KismetMathLibrary.RandomFloatInRange` 100.0 400.0)) _returnvalue_y (- _returnvalue_z 550.0))) "AlwaysSpawn" "OverrideRootScale" null null))
  (`KismetArrayLibrary.Array_Add` _platforms_2 _returnvalue)
  (for _ (range (+ (`/Game/ThirdPersonBP/Blueprints/ThirdPersonCharacter.Difficulty` (`self.TPC`)) 1))
    (bind _returnvalue_2 (`|SpawnActorFromClass` "/Game/BP_Platform.BP_Platform_C" (`KismetMathLibrary.MakeTransform` (`KismetMathLibrary.MakeVector` (+ (+ 600.0 _returnvalue_x_3) (`KismetMathLibrary.RandomFloatInRange` 100.0 400.0)) _returnvalue_y_3 _returnvalue_z_3)) "AlwaysSpawn" "OverrideRootScale" null null))
    (`KismetArrayLibrary.Array_Add` _platforms _returnvalue_2))
  (`|SpawnActorFromClass` "/Game/BP_Exit.BP_Exit_C" (`KismetMathLibrary.MakeTransform` (`KismetMathLibrary.MakeVector` (+ (+ _returnvalue_x_2 600.0) (`KismetMathLibrary.RandomFloatInRange` 100.0 400.0)) _returnvalue_y_2 _returnvalue_z_2)) "AlwaysSpawn" "OverrideRootScale" null null))

(fn `UserConstructionScript`)