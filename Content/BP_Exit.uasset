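; BP_Exit is a level exit that moves the player to a newly spawned BP_Start when a ThirdPersonCharacter overlaps it.
; The overlap first destroys the actors in the character's Dead array, all BP_Coins and all existing BP_Start actors, with validity checks on the first two.
; It then spawns a BP_Start at a fixed offset from the exit and moves the character cached at BeginPlay to that location.
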(event `self.ReceiveBeginPlay`
  (bind _returnvalue (`GameplayStatics.GetActorOfClass` "/Game/ThirdPersonBP/Blueprints/ThirdPersonCharacter.ThirdPersonCharacter_C"))
  (set `self.TPC` _returnvalue))

(event `self.ReceiveActorBeginOverlap`
  (params (OtherActor :type "Actor Object Reference"))
  (bind _returnvalue (+ (`self.K2_GetActorLocation`) (0.0 1000.0 1000.0)))
  (bind _asthird_person_character (cast `/Game/ThirdPersonBP/Blueprints/ThirdPersonCharacter` OtherActor))
  (`|ExecutionSequence`
    (:`then_0`
      (bind _dead (`/Game/ThirdPersonBP/Blueprints/ThirdPersonCharacter.Dead` _asthird_person_character))
      (`/Engine/EditorBlueprintResources/StandardMacros.IsValid` (`|GetArrayItem` _dead)
        (:`Is Valid`
          (`self.K2_DestroyActor` _dead))
        (:`Is Not Valid`
          _))
      (`/Engine/EditorBlueprintResources/StandardMacros.IsValid` "/Game/BP_Coins.BP_Coins"
        (:`Is Valid`
          (bind _outactors (`GameplayStatics.GetAllActorsOfClass` "/Game/BP_Coins.BP_Coins_C"))
          (`self.K2_DestroyActor` _outactors))
        (:`Is Not Valid`
          _))
      (bind _outactors_2 (`GameplayStatics.GetAllActorsOfClass` "/Game/BP_Start.BP_Start_C"))
      (`self.K2_DestroyActor` _outactors_2))
    (:`then_1`
      (`|SpawnActorFromClass` "/Game/BP_Start.BP_Start_C" (`KismetMathLibrary.MakeTransform` _returnvalue) "AlwaysSpawn" "OverrideRootScale" null null)
      (`self.K2_SetActorLocation` (`self.TPC`) _returnvalue false false))))

(fn `UserConstructionScript`)