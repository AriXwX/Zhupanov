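; BP_PlatformWithSpinner is a platform obstacle with a cylinder spinner that yaws in a direction chosen at random on BeginPlay.
; Each Tick it reads flags from the cached ThirdPersonCharacter: Fast cuts spin speed to a fifth, and Safe disables collision on all five cylinders.
; Collision returns to query and physics whenever Safe is off, re-applied every frame.
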(event `self.ReceiveTick`
  (params (DeltaSeconds :type "Float (single-precision)"))
  (`SceneComponent.K2_AddLocalRotation` (`self.Cylinder4`) (`KismetMathLibrary.MakeRotator` 0.0 0.0 (* (/ (stale `self.ReceiveBeginPlay` _output_get) (select `bool` (`/Game/ThirdPersonBP/Blueprints/ThirdPersonCharacter.Fast` (stale `self.ReceiveBeginPlay` _returnvalue)) :`false` 1 :`true` 5)) DeltaSeconds)) false false)
  (if (`/Game/ThirdPersonBP/Blueprints/ThirdPersonCharacter.Safe` (stale `self.ReceiveBeginPlay` _returnvalue))
    (`PrimitiveComponent.SetCollisionEnabled` (`self.Cylinder`) "NoCollision")
    (`PrimitiveComponent.SetCollisionEnabled` (`self.Cylinder1`) "NoCollision")
    (`PrimitiveComponent.SetCollisionEnabled` (`self.Cylinder2`) "NoCollision")
    (`PrimitiveComponent.SetCollisionEnabled` (`self.Cylinder3`) "NoCollision")
    (`PrimitiveComponent.SetCollisionEnabled` (`self.Cylinder4`) "NoCollision")
    (else
      (`PrimitiveComponent.SetCollisionEnabled` (`self.Cylinder`) "QueryAndPhysics")
      (`PrimitiveComponent.SetCollisionEnabled` (`self.Cylinder1`) "QueryAndPhysics")
      (`PrimitiveComponent.SetCollisionEnabled` (`self.Cylinder2`) "QueryAndPhysics")
      (`PrimitiveComponent.SetCollisionEnabled` (`self.Cylinder3`) "QueryAndPhysics")
      (`PrimitiveComponent.SetCollisionEnabled` (`self.Cylinder4`) "QueryAndPhysics"))))

(event `self.ReceiveBeginPlay`
  (bind _returnvalue (`GameplayStatics.GetActorOfClass` "/Game/ThirdPersonBP/Blueprints/ThirdPersonCharacter.ThirdPersonCharacter_C"))
  (bind _output_get (set `self.Direction` (select `int` (`KismetMathLibrary.RandomIntegerInRange` 0 1) :`0` 100 :`1` -100))))

(fn `UserConstructionScript`)